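; FishLeader is a fish pawn that swims continuously from one shared destination to the next, presumably leading other fish.
; From BeginPlay, SwimTo reads FishVector from the MyGI game instance and runs AI MoveTo toward it.
; On either success or failure it sets UpdateFishVector on the game instance, flagging that a new target is needed, then calls SwimTo again after a short delay.
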(event `self.ReceiveBeginPlay`
  (`self.SwimTo`))

(event `SwimTo`
  (bind _asmy_gi (cast `/Game/Blueprints/MyGI` (`GameplayStatics.GetGameInstance`)))
  (`|AIMoveTo` self (`/Game/Blueprints/MyGI.FishVector` _asmy_gi) null
    (:`OnSuccess`
      _)
    (:`OnFail`
      _))
  (bind _asmy_gi_2 (cast `/Game/Blueprints/MyGI` (`GameplayStatics.GetGameInstance`)))
  (set `/Game/Blueprints/MyGI.UpdateFishVector` true _asmy_gi_2)
  (`KismetSystemLibrary.Delay` 0.2)
  (`self.SwimTo`))

(event `self.ReceiveTick`
  (params (DeltaSeconds :type "Float (single-precision)")))

(fn `UserConstructionScript`
  (`parent.UserConstructionScript`))