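; Fish spawner actor that populates a box volume with a school of fish when play begins.
; It spawns one LeaderFish, then a random count of followers between a minimum and maximum, each a coin flip between the Yellow and Blue classes.
; Every fish appears at its own random point inside the Box component's scaled extent.
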(event `self.ReceiveBeginPlay`
  (bind _box (`self.Box`))
  (bind _returnvalue (`KismetMathLibrary.Conv_VectorToTransform` (`KismetMathLibrary.RandomPointInBoundingBox` (`SceneComponent.K2_GetComponentLocation` _box) (`BoxComponent.GetScaledBoxExtent` _box))))
  (`|SpawnActorFromClass` "/Game/Blueprints/Fish/Blueprints/LeaderFish.LeaderFish_C" _returnvalue "Undefined" "OverrideRootScale" null null)
  (for _ (range (+ (`KismetMathLibrary.FTrunc` (`KismetMathLibrary.RandomFloatInRange` 5.0 50.0)) 1))
    (if (`KismetMathLibrary.RandomBool`)
      (`|SpawnActorFromClass` "/Game/Blueprints/Fish/Blueprints/Yellow.Yellow_C" _returnvalue "Undefined" "OverrideRootScale" null null)
      (else
        (`|SpawnActorFromClass` "/Game/Blueprints/Fish/Blueprints/Blue.Blue_C" _returnvalue "Undefined" "OverrideRootScale" null null)))))

(fn `UserConstructionScript`)