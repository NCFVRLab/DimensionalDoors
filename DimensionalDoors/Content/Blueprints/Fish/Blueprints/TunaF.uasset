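; Follower tuna fish that continually moves toward the TunaLeader actor using AI movement.
; On BeginPlay it starts a Follow event, which looks up the leader by class and issues an AI MoveTo with that actor as target.
; Success and failure both lead to a short delay before Follow calls itself again, forming an endless chase loop without Tick.
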(event `self.ReceiveBeginPlay`
  (`self.Follow`))

(event `Follow`
  (bind _returnvalue (`GameplayStatics.GetActorOfClass` "/Game/Blueprints/Fish/Blueprints/TunaLeader.TunaLeader_C"))
  (`|AIMoveTo` self (0.0 0.0 0.0) _returnvalue
    (:`OnSuccess`
      _)
    (:`OnFail`
      _))
  (`KismetSystemLibrary.Delay` 0.2)
  (`self.Follow`))

(fn `UserConstructionScript`
  (`parent.UserConstructionScript`))