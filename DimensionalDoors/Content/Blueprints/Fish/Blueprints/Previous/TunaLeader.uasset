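; TunaLeader is a fish pawn that wanders at random through the level.
; From BeginPlay, a Move event sends it by AIMoveTo to a random reachable point within a radius of its current location.
; Success and failure both lead through a short delay back into Move, so the wandering repeats.
; Logic to spawn a TunaF at its capsule location exists but is unconnected and never runs.
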(event `self.ReceiveBeginPlay`
  (`self.Move`))

(event `Move`
  (`|AIMoveTo` self (`NavigationSystemV1.K2_GetRandomReachablePointInRadius` (`self.K2_GetActorLocation`) 500.0 null null) null
    (:`OnSuccess`
      _)
    (:`OnFail`
      _))
  (`KismetSystemLibrary.Delay` 0.2)
  (`self.Move`))

(fn `UserConstructionScript`
  (`parent.UserConstructionScript`))