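; FishFollow is a fish character that trails a FishLead actor.
; On BeginPlay it picks a random walk speed and caches the last FishLead found in the level as its Leader.
; Follow2 runs AI MoveTo toward that Leader and restarts itself after a short delay on success or failure.
; An older Follow event, which looks up a FishLead on each pass, remains but is never called.
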(event `self.ReceiveBeginPlay`
  (set `CharacterMovementComponent.MaxWalkSpeed` (`KismetMathLibrary.RandomFloatInRange` 25.0 45.0) (`self.CharacterMovement`))
  (bind _outactors (`GameplayStatics.GetAllActorsOfClass` "/Game/Blueprints/Fish/Blueprints/Previous/FishLead.FishLead_C"))
  (set `self.Leader` (`|GetArrayItem` _outactors (- (`KismetArrayLibrary.Array_Length` _outactors) 1)))
  (`self.Follow2`))

(event `Follow`
  (bind _returnvalue (`GameplayStatics.GetActorOfClass` "/Game/Blueprints/Fish/Blueprints/Previous/FishLead.FishLead_C"))
  (`|AIMoveTo` self (0.0 0.0 0.0) _returnvalue 10.0
    (:`OnSuccess`
      _)
    (:`OnFail`
      _))
  (`KismetSystemLibrary.Delay` 0.2)
  (`self.Follow`))

(event `Follow2`
  (`|AIMoveTo` self (0.0 0.0 0.0) (`self.Leader`) 10.0
    (:`OnSuccess`
      _)
    (:`OnFail`
      _))
  (`KismetSystemLibrary.Delay` 0.2)
  (`self.Follow2`))

(fn `UserConstructionScript`
  (`parent.UserConstructionScript`))