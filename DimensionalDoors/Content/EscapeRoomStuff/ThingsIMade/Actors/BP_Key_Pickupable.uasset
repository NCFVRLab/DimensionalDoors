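; A VR key actor in an escape room that motion controllers pick up and drop to solve the second puzzle.
; Overlapping OverlapThingy starts a three-second delay, and a Gate that closes on end overlap lets completion through only while open.
; Passing the gate sets SecondPuzzleComplete and calls CallPuzzle2Complete.
; Pickup disables mesh physics and attaches the key to the given component, while Drop restores physics and detaches it.
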(event `self.ReceiveActorBeginOverlap`
  (params (OtherActor :type "Actor Object Reference"))
  (if (== OtherActor (`self.OverlapThingy`))
    (`|ExecutionSequence`
      (:`then_0`
        (`KismetSystemLibrary.Delay` 3.0)
        (`/Engine/EditorBlueprintResources/StandardMacros.Gate` false :!label _label
          (:`Exit`
            (set `self.SecondPuzzleComplete` true)
            (`self.Puzzle2Complete`))))
      (:`then_1`
        (goto _label :!via `Open`)))))

(event `self.ReceiveActorEndOverlap`
  (params (OtherActor :type "Actor Object Reference"))
  (if (== OtherActor (`self.OverlapThingy`))
    (goto _label :!via `Close`)))

(event `/Game/VirtualRealityBP/Blueprints/PickupActorInterface.Pickup`
  (params (AttachTo :type "SceneComponent Object Reference"))
  (`PrimitiveComponent.SetSimulatePhysics` (`self.StaticMeshComponent`) false)
  (`SceneComponent.K2_AttachToComponent` (`self.K2_GetRootComponent`) AttachTo "None" "KeepWorld" "KeepWorld" "KeepWorld" false))

(event `/Game/VirtualRealityBP/Blueprints/PickupActorInterface.Drop`
  (`PrimitiveComponent.SetSimulatePhysics` (`self.StaticMeshComponent`) true)
  (`self.K2_DetachFromActor` "KeepWorld" "KeepWorld" "KeepWorld"))

(fn `UserConstructionScript`)